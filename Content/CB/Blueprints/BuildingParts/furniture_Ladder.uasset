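; Placeable furniture ladder building part that lets the player climb while inside its collision volume.
; On overlap, it fetches the player through PlayerInterface and, unless build mode is active, sets OnLadder and switches movement to Flying with controller-yaw rotation instead of orient-to-movement.
; Ending the overlap clears the flag and restores Walking and orient-to-movement, without checking build mode.
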(event OnComponentBeginOverlap(LadderCollision)
  (params (OverlappedComponent :type Primitive%20Component%20Object%20Reference) (OtherActor :type Actor%20Object%20Reference) (OtherComp :type Primitive%20Component%20Object%20Reference) (OtherBodyIndex :type Integer) (bFromSweep :type Boolean) (SweepResult :type Hit%20Result%20Structure%20%28by%20ref%29))
  (if (Utilities|DoesObjectImplementInterface OtherActor "/Game/CB/Blueprints/Player/PlayerInterface.PlayerInterface_C")
    (bind _player (Class|PlayerInterface|GetPlayer(Message) OtherActor))
    (if (not (Variables|/Game/CB/Blueprints/Player/Player.Player_C|GetisBuildModeActive? _player))
      (Variables|/Game/CB/Blueprints/Player/Player.Player_C|SetonLadder? _player true)
      (Pawn|Components|CharacterMovement|SetMovementMode (Variables|/Script/Engine.Character|GetCharacterMovement _player) "MOVE_Flying" 0)
      (Variables|/Script/Engine.CharacterMovementComponent|SetbOrientRotationToMovement (Variables|/Script/Engine.Character|GetCharacterMovement _player) false)
      (Variables|/Script/Engine.Pawn|SetbUseControllerRotationYaw _player true))))

(event OnComponentEndOverlap(LadderCollision)
  (params (OverlappedComponent :type Primitive%20Component%20Object%20Reference) (OtherActor :type Actor%20Object%20Reference) (OtherComp :type Primitive%20Component%20Object%20Reference) (OtherBodyIndex :type Integer))
  (if (Utilities|DoesObjectImplementInterface OtherActor "/Game/CB/Blueprints/Player/PlayerInterface.PlayerInterface_C")
    (bind _player (Class|PlayerInterface|GetPlayer(Message) OtherActor))
    (Variables|/Game/CB/Blueprints/Player/Player.Player_C|SetonLadder? _player false)
    (Pawn|Components|CharacterMovement|SetMovementMode (Variables|/Script/Engine.Character|GetCharacterMovement _player) "MOVE_Walking" 0)
    (Variables|/Script/Engine.CharacterMovementComponent|SetbOrientRotationToMovement (Variables|/Script/Engine.Character|GetCharacterMovement _player) true)
    (Variables|/Script/Engine.Pawn|SetbUseControllerRotationYaw _player false)))

(event EventBeginPlay
  (|CallParentFunction) ; This node is disabled and will not be called.\nDrag off pins to build functionality.
)

(event Collision|EventActorBeginOverlap
  (params (OtherActor :type Actor%20Object%20Reference))
  (|CallParentFunction OtherActor) ; This node is disabled and will not be called.\nDrag off pins to build functionality.
)

(event EventTick
  (params (DeltaSeconds :type Float%20%28single-precision%29))
  (|CallParentFunction DeltaSeconds) ; This node is disabled and will not be called.\nDrag off pins to build functionality.
)

(fn ConstructionScript
  (|CallParentFunction))