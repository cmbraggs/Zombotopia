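; Zombot_AI is the AI controller for the Zombot enemy, starting its attack state when it perceives the player.
; On BeginPlay it runs the Zombot_BT behavior tree.
; AI perception updates for the player character set the "attacking?" blackboard key to true if it is not already set.
; The update does not check whether the stimulus was sensed or lost, and nothing here clears the key.
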(event OnTargetPerceptionUpdated(AIPerception)
  (params (Actor :type Actor%20Object%20Reference) (Stimulus :type AI%20Stimulus%20Structure))
  (bind _returnvalue (AI|GetBlackboard 0))
  (if (and (== Actor (Game|GetPlayerCharacter 0)) (not (ScalableFloat|GetValueasBool _returnvalue (Utilities|Name|MakeLiteralName "attacking?"))))
    (AI|Components|Blackboard|SetValueasBool _returnvalue (Utilities|Name|MakeLiteralName "attacking?") true)))

(event EventBeginPlay
  (AI|RunBehaviorTree "/Game/CB/Blueprints/_AI/Data/Zombot_BT.Zombot_BT"))

(fn ConstructionScript)